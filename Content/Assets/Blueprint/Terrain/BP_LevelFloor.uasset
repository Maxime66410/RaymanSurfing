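; Procedural floor segment that builds random road tiles across seven lanes and chains to the next segment.
; On BeginPlay it random-walks adjacent lanes from LastPlaceIndex, spawning mostly basic, sometimes falling or moving floors as child actors, plus a random jewel or obstacle above them.
; A first segment spawns only FirstObject in the middle.
; It reports the last lane to BP_Generations, requests the next road when the player hits EndTrigger, then destroys itself.
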(event `self.ReceiveBeginPlay`
  ;[1 1 1] Get BP_Generation
  (bind _returnvalue (`GameplayStatics.GetActorOfClass` "/Game/Assets/Blueprint/Terrain/BP_Generations.BP_Generations_C"))
  (set `self.GenerationCast` _returnvalue)
  (`KismetSystemLibrary.Delay` 0.1)
  (if (not (`self.FirstPlace?`))
    (`self.SetSpawnPoints`)
    (`self.SetRoads`)
    (`self.SetObstacles`)
    (`self.SpawnRoads`)
    (`self.SpawnObstacles`)
    (else
      (`self.SpawnFirst?`)))
  (`self.SendInfo`))

(event `self.End Trigger.OnComponentBeginOverlap`
  (params (OverlappedComponent :type "PrimitiveComponent Object Reference") (OtherActor :type "Actor Object Reference") (OtherComp :type "PrimitiveComponent Object Reference") (OtherBodyIndex :type Integer) (bFromSweep :type Boolean) (SweepResult :type "HitResult Structure (by ref)"))
  ;[1 1 1] If player hit, Add road + Destroy this actor
  (cast `/Game/Assets/Blueprint/Players/BP_Player` OtherActor)
  (`/Game/Assets/Blueprint/Terrain/BP_Generations.AddRoad` (`self.GenerationCast`) (`SceneComponent.K2_GetComponentLocation` (`self.AttachPoint`)))
  (`KismetSystemLibrary.Delay` 2.0)
  (`self.K2_DestroyActor`))

(fn `SendInfo`
  (bind _generationcast (`self.GenerationCast`))
  (`/Engine/EditorBlueprintResources/StandardMacros.IsValid` _generationcast
    (:`Is Valid`
      (`/Game/Assets/Blueprint/Terrain/BP_Generations.ReceiveIndex` _generationcast (`self.LastPlaceIndex`)))))

(fn `SetObstacles`
  (set `self.Obstacles` (`|MakeArray` "/Game/Assets/Blueprint/Bonus/BP_GoldJewel.BP_GoldJewel_C" "/Game/Assets/Blueprint/Bonus/BP_GoldJewelSuper.BP_GoldJewelSuper_C" "/Game/Assets/Blueprint/Bonus/BP_GoldJewelMega.BP_GoldJewelMega_C" "/Game/Assets/Blueprint/Bonus/BP_Hoodmonger.BP_Hoodmonger_C" null :!type "Actor Class Reference")))

(fn `SetRoads`
  (set `self.Roads` (`|MakeArray` "/Game/Assets/Blueprint/Terrain/Floor/BP_BasicFloor.BP_BasicFloor_C" "/Game/Assets/Blueprint/Terrain/Floor/BP_FallFloor.BP_FallFloor_C" "/Game/Assets/Blueprint/Terrain/Floor/BP_MoveFloor.BP_MoveFloor_C" :!type "Actor Class Reference")))

(fn `SetSpawnPoints`
  (set `self.SpawnPoints` (`|MakeArray` (`SceneComponent.GetRelativeTransform` (`self.SpawnL2`)) (`SceneComponent.GetRelativeTransform` (`self.SpawnL1`)) (`SceneComponent.GetRelativeTransform` (`self.SpawnL`)) (`SceneComponent.GetRelativeTransform` (`self.SpawnM`)) (`SceneComponent.GetRelativeTransform` (`self.SpawnR`)) (`SceneComponent.GetRelativeTransform` (`self.SpawnR1`)) (`SceneComponent.GetRelativeTransform` (`self.SpawnR2`)))))

(fn `SpawnFirst?`
  (bind _returnvalue (`AddComponent|NODE_AddChildActorComponent-3` :`RelativeTransform` (`SceneComponent.GetRelativeTransform` (`self.SpawnM`))))
  (`ChildActorComponent.SetChildActorClass` _returnvalue (`self.FirstObject`)))

(fn `SpawnObstacles`
  (bind _obstacles (`self.Obstacles`))
  (bind _childarray (`self.ChildArray`))
  (bind (_returnvalue_location _returnvalue_rotation _returnvalue_scale) (`KismetMathLibrary.BreakTransform` (`SceneComponent.GetRelativeTransform` (`|GetArrayItem` _childarray (`KismetMathLibrary.RandomIntegerInRange` 0 (`KismetArrayLibrary.Array_LastIndex` _childarray))))))
  (bind _returnvalue (`AddComponent|NODE_AddChildActorComponent-0` :`RelativeTransform` (`KismetMathLibrary.MakeTransform` (`KismetMathLibrary.MakeVector` (.x _returnvalue_location) (.y _returnvalue_location) (+ (.z _returnvalue_location) 100.0)) _returnvalue_rotation _returnvalue_scale)))
  (`ChildActorComponent.SetChildActorClass` _returnvalue (`|GetArrayItem` _obstacles (`KismetMathLibrary.RandomIntegerInRange` 0 (`KismetArrayLibrary.Array_LastIndex` _obstacles)))))

(fn `SpawnRoads`
  (locals (lastPlace :type Integer :default 0) (`first?` :type Boolean :default true) (ToGet :type Integer))
  (bind _roads (`self.Roads`))
  (bind _lastplaceindex (`self.LastPlaceIndex`))
  (for _ (range (+ (`KismetMathLibrary.RandomIntegerInRange` 0 6) 1))
    (if (`local.first?`)
      (set `local.first?` false)
      (if (!= (`self.LastPlaceIndex`) 0)
        (set `local.ToGet` (`self.LastPlaceIndex`))
        (else
          (set `self.LastPlaceIndex` 0)
          (set `local.ToGet` (`self.LastPlaceIndex`))))
      (elif (!= (`self.LastPlaceIndex`) 6)
        (if (!= (`self.LastPlaceIndex`) 0)
          (if (`KismetMathLibrary.RandomBool`)
            (bind _output_get (set `local.ToGet` (+ _lastplaceindex 1)))
            (set `self.LastPlaceIndex` _output_get)
            (else
              (bind _output_get_2 (set `local.ToGet` (- _lastplaceindex 1)))
              (set `self.LastPlaceIndex` _output_get_2)))
          (else
            (bind _output_get_3 (set `local.ToGet` (+ (`self.LastPlaceIndex`) 1)))
            (set `self.LastPlaceIndex` _output_get_3)))
        (else
          (bind _output_get_4 (set `local.ToGet` (- (`self.LastPlaceIndex`) 1)))
          (set `self.LastPlaceIndex` _output_get_4))))
    (for (_array_element _array_index) (`self.AlreadyInPlace`)
      (if (== _array_index (`local.ToGet`))
        (if _array_element
          (set `self.IsNotAlreadyInPlace` true)
          (break))))
    (if (not (`self.IsNotAlreadyInPlace`))
      (bind _returnvalue (`AddComponent|NODE_AddChildActorComponent-2` :`RelativeTransform` (`|GetArrayItem` (`self.SpawnPoints`) (`local.ToGet`))))
      (if (`KismetMathLibrary.RandomBoolWithWeight` 0.15)
        (`ChildActorComponent.SetChildActorClass` _returnvalue (`|GetArrayItem` _roads 1))
        (elif (`KismetMathLibrary.RandomBoolWithWeight` 0.15)
          (`ChildActorComponent.SetChildActorClass` _returnvalue (`|GetArrayItem` _roads 2))
          (else
            (`ChildActorComponent.SetChildActorClass` _returnvalue (`|GetArrayItem` _roads)))))
      (`KismetArrayLibrary.Array_AddUnique` (`self.ChildArray`) _returnvalue)
      (`KismetArrayLibrary.Array_Set` (`self.AlreadyInPlace`) (`local.ToGet`) true))))

(fn `UserConstructionScript`)