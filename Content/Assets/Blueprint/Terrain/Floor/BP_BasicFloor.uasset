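; BP_BasicFloor is a terrain floor actor that randomizes its static mesh when play begins.
; A weighted coin flip favors the first mesh in ListOfAllObject's mesh list, otherwise any entry from that list is picked at random.
; Either way, the mesh component is then set to block all collision channels.
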(event `self.ReceiveBeginPlay`
  (bind _staticmesh (`self.StaticMesh`))
  (bind _listofallobject_listofstaticmesh (break `/Game/Assets/Blueprint/Terrain/Floor/ST_StaticFloorList` (`self.ListOfAllObject`)))
  (if (`KismetMathLibrary.RandomBoolWithWeight` 0.3)
    (`StaticMeshComponent.SetStaticMesh` _staticmesh (`|GetArrayItem` _listofallobject_listofstaticmesh))
    (`PrimitiveComponent.SetCollisionResponseToAllChannels` _staticmesh "ECR_Block")
    (else
      (`StaticMeshComponent.SetStaticMesh` _staticmesh (`|GetArrayItem` _listofallobject_listofstaticmesh (`KismetMathLibrary.RandomInteger` (`KismetArrayLibrary.Array_Length` _listofallobject_listofstaticmesh))))
      (`PrimitiveComponent.SetCollisionResponseToAllChannels` _staticmesh "ECR_Block"))))

(fn `UserConstructionScript`)