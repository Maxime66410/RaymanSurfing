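; BP_MoveFloor is a terrain floor actor whose static mesh starts turned sideways and eases back to a straight orientation.
; On BeginPlay it randomly sets the mesh yaw to a quarter turn left or right, then enables movement after a short delay.
; While movement is enabled, Tick uses FInterpTo to ease the relative yaw toward the default zero target.
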(event `self.ReceiveBeginPlay`
  (`SceneComponent.K2_SetRelativeRotation` (`self.StaticMesh`) (`KismetMathLibrary.MakeRotator` 0.0 0.0 (`KismetMathLibrary.SelectFloat` 90.0 -90.0 (`KismetMathLibrary.RandomBool`))) false false)
  (`KismetSystemLibrary.Delay` 2.0)
  (set `self.CanMove` true))

(event `self.ReceiveTick`
  (params (DeltaSeconds :type "Float (single-precision)"))
  (bind _staticmesh (`self.StaticMesh`))
  (bind (_relativerotation_roll _relativerotation_pitch _relativerotation_yaw) (`KismetMathLibrary.BreakRotator` (`SceneComponent.RelativeRotation` _staticmesh)))
  (set `self.Delta Seconds` DeltaSeconds)
  (if (`self.CanMove`)
    (`SceneComponent.K2_SetRelativeRotation` _staticmesh (`KismetMathLibrary.MakeRotator` 0.0 0.0 (`KismetMathLibrary.FInterpTo` _relativerotation_yaw 0.0 (`self.Delta Seconds`) 2.0)) false false)))

(fn `UserConstructionScript`)