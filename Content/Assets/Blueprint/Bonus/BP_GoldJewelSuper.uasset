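; BP_GoldJewelSuper is a gold jewel bonus pickup that awards points when BP_Player overlaps its box.
; Tick spins the static mesh at SpeedRotate and, once CanFly is set, lifts it upward, both using FInterpTo toward relative offsets.
; On pickup, it adds points through GM_RaymanSurfMode, speeds up the spin, starts the rise, plays sound, adds force feedback and destroys the box to prevent retriggering.
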(event `self.ReceiveTick`
  (params (DeltaSeconds :type "Float (single-precision)"))
  (bind _staticmesh (`self.StaticMesh`))
  (bind _staticmesh_2 (`self.StaticMesh`))
  (bind (_relativerotation_roll _relativerotation_pitch _relativerotation_yaw) (`KismetMathLibrary.BreakRotator` (`SceneComponent.RelativeRotation` _staticmesh)))
  (bind (_relativelocation_x _relativelocation_y _relativelocation_z) (`KismetMathLibrary.BreakVector` (`SceneComponent.RelativeLocation` _staticmesh_2)))
  ;[1 1 1] Animations System
  (set `self.Delta Seconds` DeltaSeconds)
  (`SceneComponent.K2_SetRelativeRotation` _staticmesh (`KismetMathLibrary.MakeRotator` 0.0 0.0 (`KismetMathLibrary.FInterpTo` _relativerotation_yaw (+ _relativerotation_yaw (`self.Speed Rotate`)) (`self.Delta Seconds`) 1.0)) false false)
  (if (`self.CanFly`)
    (`SceneComponent.K2_SetRelativeLocation` _staticmesh_2 (`KismetMathLibrary.MakeVector` 0.0 0.0 (`KismetMathLibrary.FInterpTo` _relativelocation_z (+ _relativelocation_z 500.0) (`self.Delta Seconds`) 2.0)) false false)))

(event `self.Box.OnComponentBeginOverlap`
  (params (OverlappedComponent :type "PrimitiveComponent Object Reference") (OtherActor :type "Actor Object Reference") (OtherComp :type "PrimitiveComponent Object Reference") (OtherBodyIndex :type Integer) (bFromSweep :type Boolean) (SweepResult :type "HitResult Structure (by ref)"))
  ;[1 1 1] Hit collision System
  (cast `/Game/Assets/Blueprint/Players/BP_Player` OtherActor)
  (bind _asgm_rayman_surf_mode (cast `/Game/Assets/Blueprint/GameMode/GM_RaymanSurfMode` (`GameplayStatics.GetGameMode`)))
  (`/Game/Assets/Blueprint/GameMode/GM_RaymanSurfMode.AddPointsBonus` _asgm_rayman_surf_mode 10)
  (set `self.CanFly` true)
  (set `self.Speed Rotate` 1000.0)
  (`GameplayStatics.PlaySound2D` "/Game/Assets/Audio/SFX/Bonus/SW_Data_00133.SW_Data_00133" 1.0 1.0 0.0 null null)
  (`AddComponent|NODE_AddForceFeedbackComponent-0`)
  (`ActorComponent.K2_DestroyComponent` (`self.Box`)))

(fn `UserConstructionScript`)