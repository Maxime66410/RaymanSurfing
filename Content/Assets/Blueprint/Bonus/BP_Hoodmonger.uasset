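; BP_Hoodmonger is an enemy in the Rayman surf mode that the player can defeat for bonus points or die to on contact.
; Overlapping its Head awards points through the player's game mode reference, plays a death sound and destroys the Trigger and Mesh components, leaving the actor in place.
; Overlapping its Trigger disables input and player collision, flags the game mode as finished, adds force feedback and destroys the player.
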(event `self.Head.OnComponentBeginOverlap`
  (params (OverlappedComponent :type "PrimitiveComponent Object Reference") (OtherActor :type "Actor Object Reference") (OtherComp :type "PrimitiveComponent Object Reference") (OtherBodyIndex :type Integer) (bFromSweep :type Boolean) (SweepResult :type "HitResult Structure (by ref)"))
  ;[1 1 1] Destroy Enemies
  (bind _asbp_player (cast `/Game/Assets/Blueprint/Players/BP_Player` OtherActor))
  (`ActorComponent.K2_DestroyComponent` (`self.Trigger`))
  (`/Game/Assets/Blueprint/GameMode/GM_RaymanSurfMode.AddPointsBonus` (`/Game/Assets/Blueprint/Players/BP_Player.As GM Rayman Surf Mode` _asbp_player) 20)
  (`GameplayStatics.PlaySound2D` "/Game/Assets/Audio/SFX/Hoodmonger/SC_DeathSound.SC_DeathSound" 1.0 1.0 0.0 null null)
  (`ActorComponent.K2_DestroyComponent` (`self.Mesh`)))

(event `self.Trigger.OnComponentBeginOverlap`
  (params (OverlappedComponent :type "PrimitiveComponent Object Reference") (OtherActor :type "Actor Object Reference") (OtherComp :type "PrimitiveComponent Object Reference") (OtherBodyIndex :type Integer) (bFromSweep :type Boolean) (SweepResult :type "HitResult Structure (by ref)"))
  ;[1 1 1] If Player Hit
  (bind _asbp_player (cast `/Game/Assets/Blueprint/Players/BP_Player` OtherActor))
  (`self.DisableInput` _asbp_player (`GameplayStatics.GetPlayerController` 0))
  (`self.SetFinish`)
  (`PrimitiveComponent.SetCollisionResponseToAllChannels` (`Character.CapsuleComponent` _asbp_player) "ECR_Ignore")
  (`AddComponent|NODE_AddForceFeedbackComponent-0`)
  (`ActorComponent.K2_DestroyComponent` (`self.Trigger`))
  (`self.K2_DestroyActor` _asbp_player))

(event `SetFinish`
  ;[1 1 1] Set Finish Game
  (bind _asgm_rayman_surf_mode (cast `/Game/Assets/Blueprint/GameMode/GM_RaymanSurfMode` (`GameplayStatics.GetGameMode`)))
  (set `/Game/Assets/Blueprint/GameMode/GM_RaymanSurfMode.IsFinish?` true _asgm_rayman_surf_mode))

(fn `UserConstructionScript`)