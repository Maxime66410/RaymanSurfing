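; Game mode for a Rayman surf mode that runs the score, music and in-game UI until the run ends.
; A self-rescheduling timer adds a point every 0.2 seconds until IsFinish is set, while a separate event adds bonus points.
; The HUD widget is created after a short delay if the player reference is valid.
; Finishing plays a death sound and, with a valid HUD, shows the end screen, stops music and returns to the main menu.
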(event `self.ReceiveBeginPlay`
  (`self.AddPoints`)
  (`self.GetUI`)
  (`self.PlaySound`))

(event `AddPoints`
  ;[1 1 1] Add points Auto
  (if (not (`self.IsFinish?`))
    (`/Engine/EditorBlueprintResources/StandardMacros.IncrementInt` (`self.Score`)
      (:`  `
        (`KismetSystemLibrary.K2_SetTimerDelegate` (delegate `AddPoints`) 0.2)))
    (else
      (`self.FinishGame`))))

(event `PlaySound`
  ;[1 1 1] Play Sound
  (`AudioComponent.Play` (`self.SC_RaymanFunkyBoardMusic_Cue`) 0.0))

(event `StopSound`
  ;[1 1 1] Stop Sound
  (`AudioComponent.Stop` (`self.SC_RaymanFunkyBoardMusic_Cue`)))

(event `AddPointsBonus`
  (params (Points :type Integer))
  ;[1 1 1] Add Points from bonus
  (set `self.Score` (+ (`self.Score`) Points)))

(event `GetUI`
  ;[1 1 1] Get UI
  (`KismetSystemLibrary.Delay` 0.1)
  (`/Engine/EditorBlueprintResources/StandardMacros.IsValid` (`self.BP_Players`)
    (:`Is Valid`
      (bind _returnvalue (`|CreateWidget` "/Game/Assets/Blueprint/UI/WB_InGame.WB_InGame_C" (`GameplayStatics.GetPlayerController` 0)))
      (bind _output_get (set `self.UI Game` _returnvalue))
      (`UserWidget.AddToViewport` _output_get 0))))

(event `FinishGame`
  (bind _ui_game (`self.UI Game`))
  (`GameplayStatics.PlaySound2D` "/Game/Assets/Audio/SFX/EndGame/SC_DeathSoundSFX.SC_DeathSoundSFX" 1.0 1.0 0.0 null null)
  (`/Engine/EditorBlueprintResources/StandardMacros.IsValid` _ui_game
    (:`Is Valid`
      (`/Game/Assets/Blueprint/UI/WB_InGame.LaunchEndGame` _ui_game)
      (`self.StopSound`)
      (`KismetSystemLibrary.Delay` 5.0)
      (`GameplayStatics.OpenLevel` "LVL_MainMenu"))))

(fn `UserConstructionScript`)