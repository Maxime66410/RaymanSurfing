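; BP_Player is the player character for Rayman surf mode, an auto-running lane switcher that registers itself with GM_RaymanSurfMode.
; Once started, Tick drives it forward along the control yaw and interpolates its X toward the current lane's entry in PlayerPos, gated by the game mode's finish state.
; Left/right or gamepad input steps among seven lanes, each change triggering a jump with a random style.
; Falling checks gate lane changes and jumps.
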(event `self.ReceiveBeginPlay`
  ;[1 1 1] Start
  (bind _asgm_rayman_surf_mode (cast `/Game/Assets/Blueprint/GameMode/GM_RaymanSurfMode` (`GameplayStatics.GetGameMode`)))
  (bind _output_get (set `self.As GM Rayman Surf Mode` _asgm_rayman_surf_mode))
  (set `/Game/Assets/Blueprint/GameMode/GM_RaymanSurfMode.BP_Players` self _output_get))

(event `self.ReceiveTick`
  (params (DeltaSeconds :type "Float (single-precision)"))
  ;[1 1 1] Basic Movement
  (if (`self.GameModeFinish?`)
    (set `self.Delta Seconds` DeltaSeconds)
    (if (`self.IsStart?`)
      (`self.Set Pos Player`)
      (`self.AddMovementInput` (`KismetMathLibrary.GetForwardVector` (`KismetMathLibrary.MakeRotator` 0.0 0.0 (.yaw (`self.GetControlRotation`))))))))

(event `InputAction|Left`
  (params (Key :type "Key Structure"))
  ;[1 1 1] Turn on left or right
  (:`Pressed`
    (`self.IsPlayerJump` :!label _label)
    (`self.CalculatePlayerPos` false)))

(event `InputAxis|GamePadAxis`
  (params (AxisValue :type "Float (single-precision)"))
  ;[1 1 1] Gamepad Support
  (switch `int` (`KismetMathLibrary.FTrunc` AxisValue)
    (:`-1`
      (goto _label))
    (:`1`
      ;[1 1 1] Turn on left or right
      (`self.IsPlayerJump` :!label _label_2)
      (`self.CalculatePlayerPos` true))))

(event `InputAction|Right`
  (params (Key :type "Key Structure"))
  ;[1 1 1] Turn on left or right
  (:`Pressed`
    (goto _label_2)))

(event `AutoJump`
  ;[1 1 1] Jump System
  (`self.IsNotPlayerJump` :!label _label_3)
  (`self.Jump`)
  (set `self.E_JumpStyle` (`KismetArrayLibrary.Array_Random` (`|MakeArray` "NewEnumerator0" "NewEnumerator1" :!type "/Game/Assets/Blueprint/Players/E_StyleJump Enum"))))

(event `InputAction|Jump`
  (params (Key :type "Key Structure"))
  ;[1 1 1] Jump System
  (:`Pressed`
    (goto _label_3)))

(event `self.OnLanded`
  (params (Hit :type "HitResult Structure (by ref)"))
  ;[1 1 1] Jump System
  (`self.StopJumping`))

(fn `CalculatePlayerPos`
  (params (Add :type Boolean))
  (if Add
    (if (!= (`self.WhereIsPlayer?`) 6)
      (set `self.WhereIsPlayer?` (+ (`self.WhereIsPlayer?`) 1))
      (`self.AutoJump`))
    (elif (!= (`self.WhereIsPlayer?`) 0)
      (set `self.WhereIsPlayer?` (- (`self.WhereIsPlayer?`) 1))
      (`self.AutoJump`))))

(fn `DebugMode`
  (`KismetSystemLibrary.PrintString` (`KismetStringLibrary.Concat_StrStr` "POS : " (`KismetStringLibrary.Conv_ByteToString` (`self.WhereIsPlayer?`))) true true (struct :`G` 0.66 :`B` 1.0 :`A` 1.0) 0.001)
  (`KismetSystemLibrary.PrintString` (`KismetStringLibrary.Concat_StrStr` "START? : " (`KismetStringLibrary.Conv_BoolToString` (`self.IsStart?`))) true true (struct :`G` 0.66 :`B` 1.0 :`A` 1.0) 0.001))

(fn `Set Pos Player`
  (bind (_returnvalue_x _returnvalue_y _returnvalue_z) (`KismetMathLibrary.BreakVector` (`self.K2_GetActorLocation`)))
  (for (_array_element _array_index) (`self.PlayerPos`)
    (if (== _array_index (`KismetMathLibrary.Conv_ByteToInt` (`self.WhereIsPlayer?`)))
      (`self.K2_SetActorLocation` (`KismetMathLibrary.MakeVector` (`KismetMathLibrary.FInterpTo` _returnvalue_x (.x _array_element) (`self.Delta Seconds`) (`self.Player Turn Speed`)) _returnvalue_y _returnvalue_z) true))))

(fn `UserConstructionScript`)